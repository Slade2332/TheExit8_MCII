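; Modular metro actor that randomly picks between no anomaly, an NPC-door anomaly and a blood-door anomaly.
; The Anomalías event sets TieneAnomalias on the first Teleport and Teleport2 actors cached at BeginPlay.
; The clean roll spawns three BP_Doors; anomaly rolls and ResetAnomalias only print placeholders for spawning.
; The blood-door roll leaves its own flag false, and TV, sign and light flags are only ever cleared.
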(event Custom|Anomalías
  (switch int (Math|Random|RandomIntegerinRange 0 2)
    (:0
      (Development|PrintString "No Anomalias")
      (Variables|Default|SetAnomalíaPuertaFollow false)
      (Variables|Default|SetAnomalía%20puerta%20sangrante false)
      (Variables|Default|SetAnomalía%20TV false)
      (Variables|Default|SetAnomalía%20Cartel false)
      (Variables|Default|SetAnomalíaLuces false)
      (Variables|/Game/Blueprints/Teleport.Teleport_C|SetTieneAnomalias (Utilities|Array|Get(acopy) (stale EventBeginPlay _outactors)) false)
      (Variables|/Game/Blueprints/Teleport2.Teleport2_C|SetTieneAnomalias (Utilities|Array|Get(acopy) (stale EventBeginPlay _outactors_2)) false)
      (Game|SpawnActorfromClass "/Game/Dynamic/Blueprints/TheExit8/BP_Door.BP_Door_C" (Math|Transform|MakeTransform "3102.619439,-1708.055261,-198.000005" "0.000000,180.000000,0.000000" "1.000000,1.000000,1.000000") "Undefined" "MultiplyWithRoot" 0 0)
      (Game|SpawnActorfromClass "/Game/Dynamic/Blueprints/TheExit8/BP_Door.BP_Door_C" (Math|Transform|MakeTransform "3480.049508,-1717.393462,-197.999985" "0.000000,180.000000,0.000000" "1.000000,1.000000,1.000000") "Undefined" "MultiplyWithRoot" 0 0)
      (Game|SpawnActorfromClass "/Game/Dynamic/Blueprints/TheExit8/BP_Door.BP_Door_C" (Math|Transform|MakeTransform "3825.114890,-1717.132026,194.999999" "0.000000,180.000000,0.000000" "1.000000,1.000000,1.000000") "Undefined" "MultiplyWithRoot" 0 0))
    (:1
      (Development|PrintString "Anomalía Door NPC")
      (Variables|Default|SetAnomalía%20puerta%20sangrante false)
      (Development|PrintString "Iría el nodo del spawn")
      (Variables|/Game/Blueprints/Teleport.Teleport_C|SetTieneAnomalias (Utilities|Array|Get(acopy) (stale EventBeginPlay _outactors)) true)
      (Variables|/Game/Blueprints/Teleport2.Teleport2_C|SetTieneAnomalias (Utilities|Array|Get(acopy) (stale EventBeginPlay _outactors_2)) true)
      (Variables|Default|SetAnomalíaPuertaFollow true)
      (CallFunction|ResetAnomalias))
    (:2
      (Development|PrintString "Door_Blood")
      (Variables|Default|SetAnomalíaPuertaFollow false)
      (Development|PrintString "Iría el nodo del spawn")
      (Variables|/Game/Blueprints/Teleport.Teleport_C|SetTieneAnomalias (Utilities|Array|Get(acopy) (stale EventBeginPlay _outactors)) true)
      (Variables|/Game/Blueprints/Teleport2.Teleport2_C|SetTieneAnomalias (Utilities|Array|Get(acopy) (stale EventBeginPlay _outactors_2)) true)
      (Variables|Default|SetAnomalía%20puerta%20sangrante false)
      (CallFunction|ResetAnomalias))))

(event Custom|ResetAnomalias
  (if (Variables|Default|GetAnomalíaPuertaFollow)
    (if (not (Variables|Default|GetAnomalía%20puerta%20sangrante))
      (Development|PrintString "Aqui iria el nomral"))
    (else
      (Development|PrintString "Aqui iria el nomral"))))

(event EventBeginPlay
  (Actor|GetAllActorsOfClass "/Game/Dynamic/Blueprints/TheExit8/BP_Door_NPC.BP_Door_NPC_C")
  (Actor|GetAllActorsOfClass "/Game/Dynamic/Blueprints/TheExit8/BP_Door_Blood.BP_Door_Blood_C")
  (bind _outactors (Actor|GetAllActorsOfClass "/Game/Blueprints/Teleport.Teleport_C"))
  (bind _outactors_2 (Actor|GetAllActorsOfClass "/Game/Blueprints/Teleport2.Teleport2_C")))

(event Collision|EventActorBeginOverlap
  (params (OtherActor :type Actor%20Object%20Reference)))

(event EventTick
  (params (DeltaSeconds :type Float%20%28single-precision%29)))

(fn ConstructionScript)