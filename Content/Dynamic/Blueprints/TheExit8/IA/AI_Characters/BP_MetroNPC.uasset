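; BP_MetroNPC is a hostile metro NPC that detects the player and restarts the MetroCDMX level on contact.
; Pawn sensing sets the HasSeenPlayer blackboard key and plays audio once, while a retriggerable delay clears sight and Tick fades the audio out.
; Sphere overlap plays a fade sequence and death sound before reloading.
; The construction script makes the modular body meshes follow the main mesh's pose.
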(event OnSeePawn(PawnSensing)
  (params (Pawn :type Pawn%20Object%20Reference))
  (Utilities|Casting|CastToBP_ThirdPersonCharacter Pawn)
  (Utilities|FlowControl|Sequence
    (:then_0
      (Variables|Default|SetCan%20See%20Enemy true)
      (AI|Components|Blackboard|SetValueasBool (AI|GetBlackboard (AI|GetAIController self)) (Utilities|Name|MakeLiteralName "HasSeenPlayer") true)
      (Utilities|FlowControl|DoOnce false
        (:Completed
          (Audio|Components|Audio|Play (Variables|Default|GetAudio) 0.0))))
    (:then_1
      (Utilities|FlowControl|RetriggerableDelay 0.6)
      (Variables|Default|SetCan%20See%20Enemy false))))

(event OnComponentBeginOverlap(Sphere)
  (params (OverlappedComponent :type Primitive%20Component%20Object%20Reference) (OtherActor :type Actor%20Object%20Reference) (OtherComp :type Primitive%20Component%20Object%20Reference) (OtherBodyIndex :type Integer) (bFromSweep :type Boolean) (SweepResult :type Hit%20Result%20Structure%20%28by%20ref%29))
  (Utilities|Casting|CastToBP_ThirdPersonCharacter OtherActor)
  (bind _returnvalue (Sequencer|Player|CreateLevelSequencePlayer "/Game/Dynamic/Levels/FadeIn_Transition.FadeIn_Transition"))
  (Sequencer|Player|Play _returnvalue :!class /Script/MovieScene.MovieSceneSequencePlayer)
  (Audio|PlaySound2D "/Game/Dynamic/Sonidos/Death.Death" 1.0 1.0 0.0 0 0)
  (Utilities|FlowControl|Delay 3.35)
  (Game|OpenLevel(byName) "MetroCDMX"))

(event EventBeginPlay
  ;[1 1 1] Create audio reference
  (bind _returnvalue (AddComponent|AddAudioComponent false))
  (Audio|Components|Audio|Stop _returnvalue)
  (Variables|Default|SetAudio _returnvalue))

(event Collision|EventActorBeginOverlap
  (params (OtherActor :type Actor%20Object%20Reference)))

(event EventTick
  (params (DeltaSeconds :type Float%20%28single-precision%29))
  (if (Variables|Default|GetCan%20See%20Enemy)
    (Utilities|FlowControl|Delay 0.4)
    (if (not (Variables|Default|GetCan%20See%20Enemy))
      (Audio|Components|Audio|FadeOut (Variables|Default|GetAudio) 5.0 0.0 "Linear" :!class /Script/Engine.AudioComponent)
      (Utilities|FlowControl|DoOnce false) ; enters at Reset
    )))

(fn ConstructionScript
  (Components|SkinnedMesh|SetLeaderPoseComponent (Variables|Default|GetTorso) (Variables|Character|GetMesh) false false))